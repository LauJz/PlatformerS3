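; Pickup actor for a paper, apparently for the tutorial, that the player can collect.
; Its Trigger shows the Widget component on begin overlap and hides it on end overlap, with no filter on the overlapping actor.
; The Interaction event sets HasPaper on the player's BP_ThirdPersonCharacter, makes the widget visible through a DoOnce, then destroys the actor.
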(event `self.Trigger.OnComponentBeginOverlap`
  (params (OverlappedComponent :type "PrimitiveComponent Object Reference") (OtherActor :type "Actor Object Reference") (OtherComp :type "PrimitiveComponent Object Reference") (OtherBodyIndex :type Integer) (bFromSweep :type Boolean) (SweepResult :type "HitResult Structure (by ref)"))
  ;[0.6427 1 0.549] Widget Visibility
  (`SceneComponent.SetHiddenInGame` (`self.Widget`) false false))

(event `self.Trigger.OnComponentEndOverlap`
  (params (OverlappedComponent :type "PrimitiveComponent Object Reference") (OtherActor :type "Actor Object Reference") (OtherComp :type "PrimitiveComponent Object Reference") (OtherBodyIndex :type Integer))
  ;[0.6427 1 0.549] Widget Visibility
  (`SceneComponent.SetHiddenInGame` (`self.Widget`) true false))

(event `/Game/BP_Implemented/BPI_Interaction.Interaction`
  (params (ItemClass :type "Actor Class Reference") (ItemIcon :type "Texture2D Object Reference") (StackAmount :type Integer))
  (`|ExecutionSequence`
    (:`then_0`
      (bind _asbp_third_person_character (cast `/Game/ThirdPerson/Blueprints/BP_ThirdPersonCharacter` (`GameplayStatics.GetPlayerCharacter` 0)))
      (set `/Game/ThirdPerson/Blueprints/BP_ThirdPersonCharacter.HasPaper` true _asbp_third_person_character)
      (`/Engine/EditorBlueprintResources/StandardMacros.DoOnce` false
        (:`Completed`
          (`SceneComponent.SetVisibility` (`self.Widget`) true false))))
    (:`then_1`
      (`self.K2_DestroyActor`))))

(fn `UserConstructionScript`)