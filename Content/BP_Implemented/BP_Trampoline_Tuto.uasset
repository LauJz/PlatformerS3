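; BP_Trampoline_Tuto is a trampoline, apparently for a tutorial, that launches the player character upward and shows a widget while something overlaps its trigger.
; A hit on the cube by BP_ThirdPersonCharacter restarts a timeline that animates the "Bounce" material parameter.
; An event track on that timeline calls LaunchCharacter with a fixed vertical velocity, overriding XY and Z so horizontal momentum is cleared.
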(event `self.Trigger.OnComponentBeginOverlap`
  (params (OverlappedComponent :type "PrimitiveComponent Object Reference") (OtherActor :type "Actor Object Reference") (OtherComp :type "PrimitiveComponent Object Reference") (OtherBodyIndex :type Integer) (bFromSweep :type Boolean) (SweepResult :type "HitResult Structure (by ref)"))
  ;[0.6427 1 0.549] Widget Visibility
  (`SceneComponent.SetHiddenInGame` (`self.Widget`) false false))

(event `self.Trigger.OnComponentEndOverlap`
  (params (OverlappedComponent :type "PrimitiveComponent Object Reference") (OtherActor :type "Actor Object Reference") (OtherComp :type "PrimitiveComponent Object Reference") (OtherBodyIndex :type Integer))
  ;[0.6427 1 0.549] Widget Visibility
  (`SceneComponent.SetHiddenInGame` (`self.Widget`) true false))

(event `self.Cube.OnComponentHit`
  (params (HitComponent :type "PrimitiveComponent Object Reference") (OtherActor :type "Actor Object Reference") (OtherComp :type "PrimitiveComponent Object Reference") (NormalImpulse :type "Vector Structure") (Hit :type "HitResult Structure (by ref)"))
  (bind _asbp_third_person_character (cast `/Game/ThirdPerson/Blueprints/BP_ThirdPersonCharacter` OtherActor))
  (`self.Move Trampoline` _asbp_third_person_character))

(event `Move Trampoline`
  (params (PlayerRef :type "Character Object Reference"))
  (bind (_direction _beta) (`Timeline|Timeline_Trampoline` :!via `PlayFromStart`)
    (:`Update`
      (`MeshComponent.SetScalarParameterValueOnMaterials` (`self.Cube`) "Bounce" _beta))
    (:`NewTrack_0`
      (`Character.LaunchCharacter` PlayerRef (0.0 0.0 1000.0) true true))))

(fn `UserConstructionScript`)