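; BP_PaperCollected is an interactable spot that displays the collected papers once the player has all three.
; Trigger overlap shows and hides the prompt Widget, without filtering which actor overlaps.
; The Interaction event checks PlayerHas3Papers and that player 0 is BP_ThirdPersonCharacter, then makes the 3Papers mesh visible and assigns it the paper static mesh.
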(event `self.Trigger.OnComponentBeginOverlap`
  (params (OverlappedComponent :type "PrimitiveComponent Object Reference") (OtherActor :type "Actor Object Reference") (OtherComp :type "PrimitiveComponent Object Reference") (OtherBodyIndex :type Integer) (bFromSweep :type Boolean) (SweepResult :type "HitResult Structure (by ref)"))
  ;[0.6427 1 0.549] Widget Visibility
  (`SceneComponent.SetHiddenInGame` (`self.Widget`) false false))

(event `self.Trigger.OnComponentEndOverlap`
  (params (OverlappedComponent :type "PrimitiveComponent Object Reference") (OtherActor :type "Actor Object Reference") (OtherComp :type "PrimitiveComponent Object Reference") (OtherBodyIndex :type Integer))
  ;[0.6427 1 0.549] Widget Visibility
  (`SceneComponent.SetHiddenInGame` (`self.Widget`) true false))

(event `/Game/BP_Implemented/BPI_Interaction.Interaction`
  (if (`self.PlayerHas3Papers?`)
    (cast `/Game/ThirdPerson/Blueprints/BP_ThirdPersonCharacter` (`GameplayStatics.GetPlayerCharacter` 0))
    (`SceneComponent.SetVisibility` (`self.3 Papers`) true false)
    (`StaticMeshComponent.SetStaticMesh` (`self.3 Papers`) "/Game/Fantastic_Village_Pack/meshes/props/deco/SM_PROP_paper_GAME2.SM_PROP_paper_GAME2")))

(fn `UserConstructionScript`)